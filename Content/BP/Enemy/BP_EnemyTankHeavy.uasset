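; BP_EnemyTankHeavy is the heavy enemy tank variant, a slow 2D flipbook character that fires slow projectiles.
; Its construction script sets type, health, walk speed, moving and frozen flipbooks, and the projectile template.
; On any damage, a FlipFlop alternates the sprite between two green tints as hit feedback.
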(event `self.ReceiveAnyDamage`
  (params (Damage :type "Float (single-precision)") (DamageType :type "DamageType Object Reference") (InstigatedBy :type "Controller Object Reference") (DamageCauser :type "Actor Object Reference"))
  (bind _sprite (`self.Sprite`))
  (`/Engine/EditorBlueprintResources/StandardMacros.FlipFlop`
    (:`A`
      (`PaperFlipbookComponent.SetSpriteColor` _sprite (struct :`R` 0.030997 :`G` 0.208333 :`A` 1.0)))
    (:`B`
      (`PaperFlipbookComponent.SetSpriteColor` _sprite (struct :`R` 0.108108 :`G` 0.333333 :`B` 0.016598 :`A` 1.0)))))

(fn `UserConstructionScript`
  (set `self.MovingFlipbook` "/Game/Spites/Flipbooks/Enemies/EnemyHeavy.EnemyHeavy")
  (`PaperFlipbookComponent.SetFlipbook` (`self.Sprite`) "/Game/Spites/Flipbooks/Enemies/EnemyHeavy.EnemyHeavy")
  (set `CharacterMovementComponent.MaxWalkSpeed` 50.0 (`self.CharacterMovement`))
  (set `self.TankType` "Heavy")
  (set `self.Health` 4.0)
  (set `self.FrozenFlipbook` "/Game/Spites/Flipbooks/Enemies/EnemyHeavyIdle.EnemyHeavyIdle")
  (set `self.ProjectileTemplate` "/Game/BP/Framework/BP_EnemyProjectileSlow.BP_EnemyProjectileSlow_C"))