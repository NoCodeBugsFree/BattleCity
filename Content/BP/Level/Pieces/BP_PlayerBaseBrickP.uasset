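; BP_PlayerBaseBrickP is a level piece, apparently part of the player base wall, that projectiles can knock out.
; On AnyDamage it ignores any damage causer that is not a Projectile, then branches on PieceType.
; Brick falls to any projectile, while Steel falls only to piercing ones.
; A knocked-out piece is not destroyed: its render component is hidden and its collision disabled.
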(event `self.ReceiveAnyDamage`
  (params (Damage :type "Float (single-precision)") (DamageType :type "DamageType Object Reference") (InstigatedBy :type "Controller Object Reference") (DamageCauser :type "Actor Object Reference"))
  (bind _rendercomponent (`self.RenderComponent`))
  (bind _rendercomponent_2 (`self.RenderComponent`))
  (bind _asprojectile (cast `Projectile` DamageCauser))
  ;[1 1 1] Brick
  (if (`|EnumEquality` (`self.PieceType`) "Brick")
    ;;[1 0.09106 0] hide the sprite and disable collision
    (`SceneComponent.SetVisibility` _rendercomponent_2 false false)
    (`PrimitiveComponent.SetCollisionEnabled` _rendercomponent_2 "NoCollision")
    (else
      ;[1 1 1] Steel
      (if (and (`Projectile.IsPiercing` _asprojectile) (`|EnumEquality` (`self.PieceType`) "Steel"))
        ;;[1 0.09106 0] hide the sprite and disable collision
        (`SceneComponent.SetVisibility` _rendercomponent false false)
        (`PrimitiveComponent.SetCollisionEnabled` _rendercomponent "NoCollision")))))

(fn `UserConstructionScript`
  (`parent.UserConstructionScript`))