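; BP_IceP is an ice level piece that makes the player tank slide while it stands on the ice.
; Overlapping the render component turns on the tank's IceSliding state.
; When an overlap ends, sliding turns off only if the tank's capsule overlaps no other ice piece, so crossing between adjacent tiles keeps it sliding.
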(event `self.RenderComponent.OnComponentBeginOverlap`
  (params (OverlappedComponent :type "PrimitiveComponent Object Reference") (OtherActor :type "Actor Object Reference") (OtherComp :type "PrimitiveComponent Object Reference") (OtherBodyIndex :type Integer) (bFromSweep :type Boolean) (SweepResult :type "HitResult Structure (by ref)"))
  ;[0 0.1599 1] Icing
  ;;[0 0.06912 1] start sliding
  (bind _asbp_player_tank (cast `/Game/BP/Framework/BP_PlayerTank` OtherActor))
  (`PlayerTank.IceSliding` _asbp_player_tank true))

(event `self.RenderComponent.OnComponentEndOverlap`
  (params (OverlappedComponent :type "PrimitiveComponent Object Reference") (OtherActor :type "Actor Object Reference") (OtherComp :type "PrimitiveComponent Object Reference") (OtherBodyIndex :type Integer))
  ;[0 0.1599 1] Icing
  (bind _asbp_player_tank (cast `/Game/BP/Framework/BP_PlayerTank` OtherActor))
  ;;[1 0.09106 0] sliding is over only when no other ice is overlapped
  (if (== (`KismetArrayLibrary.Array_Length` (`PrimitiveComponent.GetOverlappingActors` (`Character.CapsuleComponent` _asbp_player_tank) "BP_IceP_C")) 0)
    (`PlayerTank.IceSliding` _asbp_player_tank false)))

(fn `UserConstructionScript`
  (`parent.UserConstructionScript`))