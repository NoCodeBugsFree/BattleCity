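; BP_BrickP is a destructible level piece that reacts to projectile hits.
; On AnyDamage it ignores causers that are not Projectiles, then destroys itself if its PieceType is Brick.
; Steel pieces are destroyed only by piercing projectiles.
; Its construction script only runs the parent's.
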(event `self.ReceiveAnyDamage`
  (params (Damage :type "Float (single-precision)") (DamageType :type "DamageType Object Reference") (InstigatedBy :type "Controller Object Reference") (DamageCauser :type "Actor Object Reference"))
  (bind _asprojectile (cast `Projectile` DamageCauser))
  ;[1 1 1] Brick
  (if (`|EnumEquality` (`self.PieceType`) "Brick")
    (`self.K2_DestroyActor`)
    (else
      ;[1 1 1] Steel
      (if (and (`Projectile.IsPiercing` _asprojectile) (`|EnumEquality` (`self.PieceType`) "Steel"))
        (`self.K2_DestroyActor`)))))

(fn `UserConstructionScript`
  (`parent.UserConstructionScript`))