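; Player base level actor, built with eight child actor slots for brick pieces.
; Its construction script sets every slot's class to BP_PlayerBaseBrickP and assigns the brick, steel and dead-base sprite variables.
; The file holds only this setup, with no logic for swapping sprites or handling destruction.
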(fn `UserConstructionScript`
  (set `self.BaseDead` "/Game/Spites/Flipbooks/Pickups/BaseDead.BaseDead")
  (set `self.SteelSprite` "/Game/Spites/LevelGeometry/PS_Steel.PS_Steel")
  (set `self.BrickSprite` "/Game/Spites/LevelGeometry/PS_Brick.PS_Brick")
  (`ChildActorComponent.SetChildActorClass` (`self.ChildActor`) "/Game/BP/Level/Pieces/BP_PlayerBaseBrickP.BP_PlayerBaseBrickP_C")
  (`ChildActorComponent.SetChildActorClass` (`self.ChildActor2`) "/Game/BP/Level/Pieces/BP_PlayerBaseBrickP.BP_PlayerBaseBrickP_C")
  (`ChildActorComponent.SetChildActorClass` (`self.ChildActor3`) "/Game/BP/Level/Pieces/BP_PlayerBaseBrickP.BP_PlayerBaseBrickP_C")
  (`ChildActorComponent.SetChildActorClass` (`self.ChildActor4`) "/Game/BP/Level/Pieces/BP_PlayerBaseBrickP.BP_PlayerBaseBrickP_C")
  (`ChildActorComponent.SetChildActorClass` (`self.ChildActor5`) "/Game/BP/Level/Pieces/BP_PlayerBaseBrickP.BP_PlayerBaseBrickP_C")
  (`ChildActorComponent.SetChildActorClass` (`self.ChildActor6`) "/Game/BP/Level/Pieces/BP_PlayerBaseBrickP.BP_PlayerBaseBrickP_C")
  (`ChildActorComponent.SetChildActorClass` (`self.ChildActor7`) "/Game/BP/Level/Pieces/BP_PlayerBaseBrickP.BP_PlayerBaseBrickP_C")
  (`ChildActorComponent.SetChildActorClass` (`self.ChildActor1`) "/Game/BP/Level/Pieces/BP_PlayerBaseBrickP.BP_PlayerBaseBrickP_C"))