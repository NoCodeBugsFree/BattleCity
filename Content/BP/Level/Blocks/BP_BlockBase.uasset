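; BP_BlockBase is a base level block built from four child actor piece components.
; Its construction script switches on PieceType (Brick, Steel, Ice, Wood or Water) and assigns the matching piece Blueprint class to all four child actors.
; The event graph holds only disabled default nodes, so this Blueprint adds no runtime logic of its own.
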(fn `UserConstructionScript`
  (switch `EPieceType` (`self.PieceType`)
    (:`Brick`
      (`ChildActorComponent.SetChildActorClass` (`self.Piece02`) "/Game/BP/Level/Pieces/BP_BrickP.BP_BrickP_C")
      (`ChildActorComponent.SetChildActorClass` (`self.Piece03`) "/Game/BP/Level/Pieces/BP_BrickP.BP_BrickP_C")
      (`ChildActorComponent.SetChildActorClass` (`self.Piece04`) "/Game/BP/Level/Pieces/BP_BrickP.BP_BrickP_C")
      (`ChildActorComponent.SetChildActorClass` (`self.Piece01`) "/Game/BP/Level/Pieces/BP_BrickP.BP_BrickP_C"))
    (:`Steel`
      (`ChildActorComponent.SetChildActorClass` (`self.Piece02`) "/Game/BP/Level/Pieces/BP_SteelP.BP_SteelP_C")
      (`ChildActorComponent.SetChildActorClass` (`self.Piece03`) "/Game/BP/Level/Pieces/BP_SteelP.BP_SteelP_C")
      (`ChildActorComponent.SetChildActorClass` (`self.Piece04`) "/Game/BP/Level/Pieces/BP_SteelP.BP_SteelP_C")
      (`ChildActorComponent.SetChildActorClass` (`self.Piece01`) "/Game/BP/Level/Pieces/BP_SteelP.BP_SteelP_C"))
    (:`Ice`
      (`ChildActorComponent.SetChildActorClass` (`self.Piece02`) "/Game/BP/Level/Pieces/BP_IceP.BP_IceP_C")
      (`ChildActorComponent.SetChildActorClass` (`self.Piece03`) "/Game/BP/Level/Pieces/BP_IceP.BP_IceP_C")
      (`ChildActorComponent.SetChildActorClass` (`self.Piece04`) "/Game/BP/Level/Pieces/BP_IceP.BP_IceP_C")
      (`ChildActorComponent.SetChildActorClass` (`self.Piece01`) "/Game/BP/Level/Pieces/BP_IceP.BP_IceP_C"))
    (:`Wood`
      (`ChildActorComponent.SetChildActorClass` (`self.Piece02`) "/Game/BP/Level/Pieces/BP_WoodP.BP_WoodP_C")
      (`ChildActorComponent.SetChildActorClass` (`self.Piece03`) "/Game/BP/Level/Pieces/BP_WoodP.BP_WoodP_C")
      (`ChildActorComponent.SetChildActorClass` (`self.Piece04`) "/Game/BP/Level/Pieces/BP_WoodP.BP_WoodP_C")
      (`ChildActorComponent.SetChildActorClass` (`self.Piece01`) "/Game/BP/Level/Pieces/BP_WoodP.BP_WoodP_C"))
    (:`Water`
      (`ChildActorComponent.SetChildActorClass` (`self.Piece02`) "/Game/BP/Level/Pieces/BP_WaterP.BP_WaterP_C")
      (`ChildActorComponent.SetChildActorClass` (`self.Piece03`) "/Game/BP/Level/Pieces/BP_WaterP.BP_WaterP_C")
      (`ChildActorComponent.SetChildActorClass` (`self.Piece04`) "/Game/BP/Level/Pieces/BP_WaterP.BP_WaterP_C")
      (`ChildActorComponent.SetChildActorClass` (`self.Piece01`) "/Game/BP/Level/Pieces/BP_WaterP.BP_WaterP_C"))))