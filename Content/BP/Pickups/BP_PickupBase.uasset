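; BP_PickupBase is the base Blueprint for pickups, with a PickupType that selects among bomb, clock, helmet, life, shovel and star variants.
; Its construction script switches on PickupType and assigns the matching flipbook to RenderComponent, so each instance displays the sprite animation for its type.
; The graph sets only the visual and contains no collection or effect logic.
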(fn `UserConstructionScript`
  (switch `EPickupType` (`self.PickupType`)
    (:`PT_Bomb`
      (`PaperFlipbookComponent.SetFlipbook` (`self.RenderComponent`) "/Game/Spites/Flipbooks/Pickups/FB_Bomb.FB_Bomb"))
    (:`PT_Clock`
      (`PaperFlipbookComponent.SetFlipbook` (`self.RenderComponent`) "/Game/Spites/Flipbooks/Pickups/FB_Clock.FB_Clock"))
    (:`PT_Helmet`
      (`PaperFlipbookComponent.SetFlipbook` (`self.RenderComponent`) "/Game/Spites/Flipbooks/Pickups/FB_Helmet.FB_Helmet"))
    (:`PT_Life`
      (`PaperFlipbookComponent.SetFlipbook` (`self.RenderComponent`) "/Game/Spites/Flipbooks/Pickups/FB_Life.FB_Life"))
    (:`PT_Shovel`
      (`PaperFlipbookComponent.SetFlipbook` (`self.RenderComponent`) "/Game/Spites/Flipbooks/Pickups/FB_Shovel.FB_Shovel"))
    (:`PT_Star`
      (`PaperFlipbookComponent.SetFlipbook` (`self.RenderComponent`) "/Game/Spites/Flipbooks/Pickups/FB_Star.FB_Star"))))